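; BP_PhysicsPickup is an interactable physics cube that the player can pick up and drop through interface events.
; On interact, if the player is not already holding something, it sets IsHolding, turns off physics and collision, and snaps the Cube to the player's Arrow1 component.
; On drop, it detaches keeping its world transform and restores physics and collision, without clearing IsHolding itself.
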(event EventINTInteract
  (params (PlayerRef :type BP%20Player%20Object%20Reference))
  (bind _cube (Variables|Default|GetCube))
  ;[1 1 1] Pick Up
  (if (not (Variables|/Game/Player/BP_Player.BP_Player_C|GetisHolding? PlayerRef))
    (Variables|/Game/Player/BP_Player.BP_Player_C|SetisHolding? PlayerRef true)
    (Physics|SetSimulatePhysics _cube false)
    (Collision|SetCollisionEnabled _cube "NoCollision")
    (Transformation|AttachComponentToComponent (Variables|Default|GetCube) (Variables|/Game/Player/BP_Player.BP_Player_C|GetArrow1 PlayerRef) "None" "SnapToTarget" "KeepRelative" "KeepRelative" true)))

(event EventINTDrop
  (bind _cube (Variables|Default|GetCube))
  ;[1 1 1] Drop
  (Transformation|DetachFromActor "KeepWorld" "KeepWorld" "KeepWorld")
  (Physics|SetSimulatePhysics _cube true)
  (Collision|SetCollisionEnabled _cube "QueryAndPhysics"))

(fn ConstructionScript)